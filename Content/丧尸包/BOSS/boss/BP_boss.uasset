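; Boss Blueprint that provides an electrocution visual effect, flashing a skeleton over a blacked-out body.
; Ce_开启电击 starts a looping timer, saved in 被电击句柄, that blinks custom depth on the 骨架双手砸被电击 skeleton component and sets the Boss material to pure black.
; Ce_初始材质 restores the original material but does not clear the timer.
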(event Custom|Ce_初始材质
  (Rendering|Material|SetMaterial (Variables|Default|Getboss) 0 "/Game/丧尸包/BOSS/boss/MI__53_.MI__53_"))

(event Custom|Ce_改材质
  (bind _骨架_双手砸被电击 (Variables|Default|Get骨架_双手砸被电击))
  (Utilities|FlowControl|Sequence
    (:then_0
      (Rendering|SetRenderCustomDepth _骨架_双手砸被电击 false)
      (Utilities|FlowControl|Delay 0.1)
      (Rendering|SetRenderCustomDepth _骨架_双手砸被电击 true))
    (:then_1
      (Rendering|Material|SetMaterial (Variables|Default|Getboss) 0 "/Game/丧尸包/BOSS/boss/M_纯黑.M_纯黑"))))

(event Custom|Ce_开启电击
  (bind _returnvalue (Utilities|Time|SetTimerbyEvent (delegate Custom|Ce_改材质) 0.2 true))
  (Variables|Default|Set被电击句柄 _returnvalue))

(event EventBeginPlay)

(event Collision|EventActorBeginOverlap
  (params (OtherActor :type Actor%20Object%20Reference)))

(event EventTick
  (params (DeltaSeconds :type Float%20%28single-precision%29)))

(fn ConstructionScript)